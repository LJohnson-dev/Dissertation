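; Enemy pawn that chases the first player character and deals damage on reaching it.
; ChasePlayer starts on BeginPlay and uses AIMoveTo; success triggers AttackPlayer, then restarts the chase after a short delay.
; AttackPlayer applies fixed damage to BP_FirstPersonCharacter, prints a debug message and calls OnAttackFinish.
; Only move success is wired, so a failed move ends the loop.
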(event Custom|ChasePlayer
  (AI|AIMoveTo self "0, 0, 0" (Game|GetPlayerCharacter 0) 1.5e+02 false
    (:OnSuccess
      (CallFunction|AttackPlayer)
      (Utilities|FlowControl|Delay 0.1)
      (CallFunction|ChasePlayer))))

(event Custom|AttackPlayer
  (bind _asbp_first_person_character (Utilities|Casting|CastToBP_FirstPersonCharacter (Game|GetPlayerCharacter 0)))
  (Game|Damage|ApplyDamage _asbp_first_person_character 2e+01 0 0)
  (Development|PrintString "Attacked")
  (Default|CallOnAttackFinish))

(event EventBeginPlay
  (CallFunction|ChasePlayer))

(event Collision|EventActorBeginOverlap
  (params (OtherActor :type Actor%20Object%20Reference)))

(event EventTick
  (params (DeltaSeconds :type Float%20%28single-precision%29)))

(fn ConstructionScript)