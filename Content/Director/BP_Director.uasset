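; AI director that periodically scores player performance to adjust difficulty by spawning enemies, medkits and ammo.
; On a timer, Evaluate averages curve-mapped health, ammo and accuracy scores, tops enemies up to a curve-driven minimum, and queues aid at or above the optimal range.
; SpawnDanger, called at or below that range, is an empty stub.
; The FIFO queue spawns at async EQS-chosen locations, and a debug widget displays the scores.
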(event Custom|OnSpawnNextQueryFinished
  (params (QueryInstance :type Env%20Query%20Instance%20Blueprint%20Wrapper%20Object%20Reference) (QueryStatus :type EEnvQueryStatus%20Enum :default "Processing"))
  (if (Utilities|Enum|Equal(Enum) QueryStatus "Success")
    (bind (_resultlocations _returnvalue) (AI|EQS|GetQueryResultsasLocations QueryInstance))
    (if _returnvalue
      (CallFunction|SpawnQueuedActor (Utilities|Array|Get(acopy) _resultlocations))
      (if (> (Utilities|Array|Length (Variables|Default|GetSpawnQueue)) 0)
        (CallFunction|SpawnNext)))))

(event Custom|SpawnNext
  (if (> (Utilities|Array|Length (Variables|Default|GetSpawnQueue)) 0)
    (bind _returnvalue (AI|EQS|RunEQSQuery "/Game/EQS/EQS_SpawnAid.EQS_SpawnAid" (Game|Player|GetPlayerPawn 0) "RandomBest25Pct"))
    (EventDispatchers|BindEventtoOnQueryFinishedEvent _returnvalue (delegate Custom|OnSpawnNextQueryFinished))
    (Variables|Default|SetCurrentEQSQuery _returnvalue)))

(event EventBeginPlay
  (bind _gamemode (CallFunction|GetCustomGamemode self))
  (Variables|Default|SetGame%20Mode _gamemode)
  (bind _returnvalue (UserInterface|CreateWidget "/Game/Director/WBP_DirectorDebug.WBP_DirectorDebug_C" (Game|GetPlayerController 0)))
  (bind _output_get (Variables|Default|SetDebugWidget _returnvalue))
  (UserInterface|Viewport|AddtoPlayerScreen _output_get))

(event EventTick
  (params (DeltaSeconds :type Float%20%28single-precision%29))
  (bind _output_get (Variables|Default|SetEvaluationTimer (- (Variables|Default|GetEvaluationTimer) DeltaSeconds)))
  (if (<= _output_get 0.0)
    (Variables|Default|SetEvaluationTimer (Variables|Default|GetEvaluationTime))
    (CallFunction|Evaluate)
    (CallFunction|SpawnNext)
    (Default|Update (Variables|Default|GetDebugWidget) (Variables|Default|GetCurrentPlayerPerf) (CallFunction|GetHealthScore) (CallFunction|GetAmmoScore) (CallFunction|GetAccuracyScore) (Variables|Default|GetOptimalPerformanceRangeLow) (Variables|Default|GetOptimalPerformanceRangeHigh))))

(fn ConstructionScript)

(fn Evaluate
  ;[1 1 1] Could improve this to control how much each component influences the final score
  (Variables|Default|SetCurrentPlayerPerf (/ (+ (CallFunction|GetHealthScore) (CallFunction|GetAmmoScore) (CallFunction|GetAccuracyScore)) 3.0))
  (CallFunction|SpawnMinimumDanger)
  (if (<= (Variables|Default|GetCurrentPlayerPerf) (Variables|Default|GetOptimalPerformanceRangeLow))
    (CallFunction|SpawnDanger)
    (elif (>= (Variables|Default|GetCurrentPlayerPerf) (Variables|Default|GetOptimalPerformanceRangeHigh))
      (CallFunction|SpawnAid))))

(fn GetHealthScore
  ;[0.8551 0.183 1] Mapping raw player health using a curve to get a standardised health score from 0-1
  (return (Math|Curves|GetFloatValue (Variables|Default|GetHealthScoreCurve) (Default|GetPlayerHealth (Variables|Default|GetGame%20Mode)))))

(fn GetAmmoScore
  (return (Math|Curves|GetFloatValue (Variables|Default|GetAmmoScoreCurve) (Math|Conversions|ToFloat(Integer) (Default|GetPlayerAmmo (Variables|Default|GetGame%20Mode))))))

(fn SpawnAid
  (if (>= (CallFunction|GetHealthScore) (* (CallFunction|GetAmmoScore) (Math|Float|Clamp(Float) (CallFunction|GetAccuracyScore) 0.1)))
    (CallFunction|AddtoSpawnQueue "/Game/Interactables/Medkit/BP_Medkit.BP_Medkit_C")
    (else
      (CallFunction|AddtoSpawnQueue "/Game/Interactables/Ammo/BP_Ammo.BP_Ammo_C"))))

(fn SpawnMinimumDanger
  ;[0.1418 0.9203 1] ensuring minimum amount of enemies will be in the level
  (bind _enemycount (CallFunction|GetEnemyCount))
  (for _index (range _enemycount (CallFunction|GetMinEnemyCount))
    (CallFunction|AddtoSpawnQueue "/Game/Enemy/BP_EnemyAI.BP_EnemyAI_C")))

(fn GetAccuracyScore
  (bind _game_mode (Variables|Default|GetGame%20Mode))
  (bind _headshots (Default|GetHeadshots _game_mode))
  (bind _bodyshots (Default|GetBodyshots _game_mode))
  (bind _returnvalue (+ _headshots _bodyshots))
  (if (<= _returnvalue 0)
    (return 0.0)
    (else
      (return (Math|Curves|GetFloatValue (Variables|Default|GetAccuracyScoreCurve) (/ (Math|Conversions|ToFloat(Integer) _bodyshots) (Math|Conversions|ToFloat(Integer) _returnvalue)))))))

(fn GetEnemyCount
  (return (Default|GetEnemyCount (Variables|Default|GetGame%20Mode))))

(fn SpawnQueuedActor
  (params (SpawnLocation :type Vector))
  (if (> (Utilities|Array|Length (Variables|Default|GetSpawnQueue)) 0)
    (LocalVariables|SetL_Index (Utilities|Array|LastIndex (Variables|Default|GetSpawnQueue)))
    (LocalVariables|SetL_ClassToSpawn (Utilities|Array|Get(acopy) (Variables|Default|GetSpawnQueue) (LocalVariables|GetL_Index)))
    (bind _returnvalue (Game|SpawnActorfromClass (LocalVariables|GetL_ClassToSpawn) (Math|Transform|MakeTransform SpawnLocation "0, 0, 0" "1.000000,1.000000,1.000000") "Undefined" "MultiplyWithRoot" 0 0))
    (Utilities|IsValid _returnvalue
      (:Is%20Valid
        (Class|BPIDirectorActor|Spawned(Message) _returnvalue)
        (Utilities|Array|RemoveIndex (Variables|Default|GetSpawnQueue) (LocalVariables|GetL_Index))
        (EventDispatchers|UnbindallEventsfromOnQueryFinishedEvent (Variables|Default|GetCurrentEQSQuery))))))

(fn AddtoSpawnQueue
  (params (ToAdd :type Actor%20Class%20Reference))
  (Utilities|Array|Insert (Variables|Default|GetSpawnQueue) ToAdd))

(fn GetMinEnemyCount
  (return (Math|Float|Ceil (Math|Curves|GetFloatValue (Variables|Default|GetMinEnemyCurve) (* (Variables|Default|GetCurrentPlayerPerf) (CallFunction|GetAccuracyScore))))))

(fn SpawnDanger)